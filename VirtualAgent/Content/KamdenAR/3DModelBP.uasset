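; 3D model Blueprint in the KamdenAR project that carries two reference points, TopNipple and TopStairs.
; GetClosestReferencePoint takes a plane actor's location and returns a reference point's relative position with a "Nipple" or "Stairs" label.
; The choice is a Z threshold rather than a distance test: at or above TopNipple's relative Z gives Nipple, anything lower gives Stairs.
; Events and construction script are empty; leftover debug prints are disconnected.
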(event `self.ReceiveBeginPlay`)

(fn `GetClosestReferencePoint`
  (params (planeActorLocation :type "Vector Structure"))
  (returns (position :type "Vector Structure") (referencePointString :type String))
  (if (>= (.z planeActorLocation) (.z (`SceneComponent.RelativeLocation` (`self.TopNipple`))))
    (return (`SceneComponent.RelativeLocation` (`self.TopNipple`)) "Nipple")
    (else
      (return (`SceneComponent.RelativeLocation` (`self.TopStairs`)) "Stairs"))))

(fn `UserConstructionScript`)